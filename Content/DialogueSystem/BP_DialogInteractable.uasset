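; BP_DialogInteractable is an interactable that plays a dialogue sequence and can trigger follow-up events when it ends.
; Box overlap enables input and HintTrigger toggles the prompt widget.
; IA_Interact starts or advances dialogue through BP_GameMode, gated by ShouldDestroyItself, which also hides its visuals.
; On key completion after dialogue ends, it disables input, activates a linked BPI_Activable actor and optionally grants the rifle, shows quests and destroys itself.
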(event OnComponentBeginOverlap(Box)
  (params (OverlappedComponent :type Primitive%20Component%20Object%20Reference) (OtherActor :type Actor%20Object%20Reference) (OtherComp :type Primitive%20Component%20Object%20Reference) (OtherBodyIndex :type Integer) (bFromSweep :type Boolean) (SweepResult :type Hit%20Result%20Structure%20%28by%20ref%29))
  (Input|EnableInput (Game|GetPlayerController 0)))

(event OnComponentEndOverlap(Box)
  (params (OverlappedComponent :type Primitive%20Component%20Object%20Reference) (OtherActor :type Actor%20Object%20Reference) (OtherComp :type Primitive%20Component%20Object%20Reference) (OtherBodyIndex :type Integer)))

(event OnComponentBeginOverlap(HintTrigger)
  (params (OverlappedComponent :type Primitive%20Component%20Object%20Reference) (OtherActor :type Actor%20Object%20Reference) (OtherComp :type Primitive%20Component%20Object%20Reference) (OtherBodyIndex :type Integer) (bFromSweep :type Boolean) (SweepResult :type Hit%20Result%20Structure%20%28by%20ref%29))
  (if (Variables|Default|GetCanShowInputHint)
    (Rendering|SetVisibility (Variables|Default|GetWidget) true false)))

(event OnComponentEndOverlap(HintTrigger)
  (params (OverlappedComponent :type Primitive%20Component%20Object%20Reference) (OtherActor :type Actor%20Object%20Reference) (OtherComp :type Primitive%20Component%20Object%20Reference) (OtherBodyIndex :type Integer))
  (bind _widget (Variables|Default|GetWidget))
  (Utilities|IsValid _widget
    (:Is%20Valid
      (Rendering|SetVisibility _widget false false))))

(event Input|EnhancedActionEvents|EnhancedInputActionIA_Interact
  (params (ActionValue :type Boolean) (ElapsedSeconds :type Float%20%28double-precision%29) (TriggeredSeconds :type Float%20%28double-precision%29) (InputAction :type Input%20Action%20Object%20Reference :default "/Game/PlayerFolder/Input/Actions/IA_Interact.IA_Interact"))
  (bind _playerreference (Variables|Default|GetPlayerReference))
  (:Started
    (if (Variables|Default|GetShouldDestroyItself)
      (Rendering|SetVisibility (Variables|Default|GetMesh) false false)
      (Rendering|SetVisibility (Variables|Default|GetSpotLight) false false)
      (Rendering|SetVisibility (Variables|Default|GetWidget) false false)
      (if (Variables|Default|GetHasStartedDialogue)
        (Default|ShowNextDialogue (Variables|Default|GetGameModeVariable))
        (else
          (Variables|Default|SetHasStartedDialogue true)
          (Variables|/Game/Blueprints/BP_GameMode.BP_GameMode_C|SetEndofDialogue (Variables|Default|GetGameModeVariable) false)
          (Default|StartDialogue (Variables|Default|GetGameModeVariable) (Variables|Default|GetDialogueSequence))))))
  (:Completed
    (if (Variables|/Game/Blueprints/BP_GameMode.BP_GameMode_C|GetEndofDialogue (Variables|Default|GetGameModeVariable))
      (Input|DisableInput (Game|GetPlayerController 0))
      (Variables|Default|SetHasStartedDialogue false)
      (Rendering|SetVisibility (Variables|Default|GetWidget) false false)
      (Variables|Default|SetCanShowInputHint false)
      (Utilities|ActivateDoor true)
      (if (Variables|Default|GetCanPickUpRifle)
        (Default|PickUpRifle _playerreference)
        (Variables|/Game/PlayerFolder/Blueprints/BP_Player.BP_Player_C|SetRifleIsActive _playerreference true)
        (bind _returnvalue (UserInterface|CreateWidget "/Game/Blueprints/Widgets/WBP_Quests.WBP_Quests_C" (Game|GetPlayerController 0)))
        (UserInterface|Viewport|AddtoViewport _returnvalue 0)
        (if (Variables|Default|GetShouldDestroyItself)
          (Actor|DestroyActor))))))

(event Collision|EventActorBeginOverlap
  (params (OtherActor :type Actor%20Object%20Reference)))

(event EventTick
  (params (DeltaSeconds :type Float%20%28single-precision%29)))

(event EventBeginPlay
  (bind _asbp_game_mode (Utilities|Casting|CastToBP_GameMode (Game|GetGameMode))
    (:then
      (Variables|Default|SetGameModeVariable _asbp_game_mode)
      (bind _asbp_player (Utilities|Casting|CastToBP_Player (Game|GetPlayerCharacter 0)))
      (Variables|Default|SetPlayerReference _asbp_player))
    (:CastFailed
      (Development|PrintString "CastFailed"))))

(fn ConstructionScript
  (Variables|Default|SetShouldDestroyItself (Variables|Default|GetShouldDestroyItself)))