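; BP_ShotgunPickUp is a pickup actor that gives the player a shotgun.
; When the IA_Interact input starts and CanPickUpShotgun is true, it calls PickUpShotgun on PlayerReference, sets that player's CurrentItemSelection to the shotgun slot and destroys itself.
; Its graphs only read CanPickUpShotgun and PlayerReference, never setting them, and the BeginPlay, overlap and Tick events are disabled stubs.
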(event Input|EnhancedActionEvents|EnhancedInputActionIA_Interact
  (params (ActionValue :type Boolean) (ElapsedSeconds :type Float%20%28double-precision%29) (TriggeredSeconds :type Float%20%28double-precision%29) (InputAction :type Input%20Action%20Object%20Reference :default "/Game/PlayerFolder/Input/Actions/IA_Interact.IA_Interact"))
  (bind _playerreference (Variables|Default|GetPlayerReference))
  (:Started
    (if (Variables|Default|GetCanPickUpShotgun)
      (Default|PickUpShotgun _playerreference)
      (Variables|/Game/PlayerFolder/Blueprints/BP_Player.BP_Player_C|SetCurrentItemSelection _playerreference 1)
      (Actor|DestroyActor))))

(event EventBeginPlay
  (|CallParentFunction) ; This node is disabled and will not be called.\nDrag off pins to build functionality.
)

(event Collision|EventActorBeginOverlap
  (params (OtherActor :type Actor%20Object%20Reference))
  (|CallParentFunction OtherActor) ; This node is disabled and will not be called.\nDrag off pins to build functionality.
)

(event EventTick
  (params (DeltaSeconds :type Float%20%28single-precision%29))
  (|CallParentFunction DeltaSeconds) ; This node is disabled and will not be called.\nDrag off pins to build functionality.
)

(fn ConstructionScript
  (|CallParentFunction))