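; Base enemy character with health, an optional child-actor shield and a health bar widget, driven by an AIC_Enemy_Base controller.
; Health, damage and healing calls forward to BPC_DamageSystem, whose death, block and damage-response events are bound in the construction script.
; Shield flags gate the hit-reaction montage, which freezes the AI until it resumes attacking.
; Death ragdolls the mesh, stops AI logic and destroys the actor after a delay.
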(event Custom|Death
  (bind _mesh (Variables|Character|GetMesh))
  (bind _as_aic_enemy_base (Variables|Default|GetAs%20AIC%20Enemy%20Base))
  (Physics|SetSimulatePhysics _mesh true)
  (Collision|SetCollisionEnabled _mesh "QueryAndPhysics")
  (Pawn|Components|CharacterMovement|SetMovementMode (Variables|Character|GetCharacterMovement) "MOVE_None" 0)
  (Collision|SetCollisionEnabled (Variables|Collision|GetCapsuleComponent) "NoCollision")
  (Variables|Default|SetbIsEnemyDead true)
  (AI|Logic|StopLogic (Variables|/Script/AIModule.AIController|GetBrainComponent _as_aic_enemy_base) "")
  (Default|SetStateasDead _as_aic_enemy_base)
  (Utilities|FlowControl|Delay 2.0)
  (Actor|DestroyActor self))

(event Custom|DamageResponse
  (params (DamageResponse :type E_DamageResponse%20Enum :default "NewEnumerator0"))
  (bind _as_aic_enemy_base (Variables|Default|GetAs%20AIC%20Enemy%20Base))
  ;[1 1 1] If i want to apply damage trigger animation to all enemies when being hit later on
  (bind _output_get (Variables|/Game/EnemyFolder/BP_Shield.BP_Shield_C|SetCanPlayHitReaction (Variables|Default|GetShieldReference) (Variables|Features|GetShouldGetStunned)))
  (if _output_get
    (if (Variables|/Game/EnemyFolder/BP_Shield.BP_Shield_C|GetPlayHitReaction (Variables|Default|GetShieldReference))
      (Components|Movement|StopMovementImmediately (Variables|Character|GetCharacterMovement))
      (Default|SetStateasFrozen (Variables|Default|GetAs%20AIC%20Enemy%20Base))
      (Animation|Montage|PlayMontage (Variables|Character|GetMesh) (Variables|Features|GetHitReactionAnimation)
        (:OnCompleted
          _)
        (:OnInterrupted
          _))
      (Default|SetStateasAttacking _as_aic_enemy_base (Variables|/Game/EnemyFolder/AIControllers/AIC_Enemy_Base.AIC_Enemy_Base_C|GetAttackTarget _as_aic_enemy_base)))))

(event Custom|Blocked
  (Development|PrintString "Blocked"))

(event EventBeginPlay
  (bind _asaic_enemy_base (Utilities|Casting|CastToAIC_Enemy_Base (AI|GetAIController self)))
  (Variables|Default|SetAs%20AIC%20Enemy%20Base _asaic_enemy_base)
  (bind _returnvalue (UserInterface|CreateWidget "/Game/DamageSystem/WBP_HealthBar.WBP_HealthBar_C" 0 self))
  (UserInterface|SetWidget (Variables|Default|GetHealthBar) _returnvalue))

(fn ConstructionScript
  (bind _bpc_damagesystem (Variables|Default|GetBPC_DamageSystem))
  (CallFunction|Enable/DisableShield)
  (bind _asbp_shield (Utilities|Casting|CastToBP_Shield (Variables|/Script/Engine.ChildActorComponent|GetChildActor (Variables|Default|GetBP_Shield))))
  (Variables|Default|SetShieldReference _asbp_shield)
  (EventDispatchers|BindEventtoOnDeath _bpc_damagesystem (EventDispatchers|CreateEvent :!event Custom|Death))
  (EventDispatchers|BindEventtoOnBlocked _bpc_damagesystem (EventDispatchers|CreateEvent :!event Custom|Blocked))
  (EventDispatchers|BindEventtoOnDamageResponse _bpc_damagesystem (EventDispatchers|CreateEvent :!event Custom|DamageResponse))
  (bind _asaic_enemy_base (Utilities|Casting|CastToAIC_Enemy_Base (AI|GetAIController self)))
  (Variables|Default|SetAs%20AIC%20Enemy%20Base _asaic_enemy_base))

(fn Enable/DisableShield
  (bind _bp_shield (Variables|Default|GetBP_Shield))
  (bind _childactor (Variables|/Script/Engine.ChildActorComponent|GetChildActor _bp_shield))
  (if (Variables|Features|GetbShouldHaveShield)
    (Rendering|SetVisibility _bp_shield true false)
    (Collision|SetActorEnableCollision _childactor true)
    (else
      (Rendering|SetVisibility _bp_shield false false)
      (Collision|SetActorEnableCollision _childactor false))))

(fn GetCurrentHealth
  (return (Variables|/Game/DamageSystem/BPC_DamageSystem.BPC_DamageSystem_C|GetHealth (Variables|Default|GetBPC_DamageSystem))))

(fn GetIdealRange
  (return 1.5e+02 3.5e+02))

(fn GetMaxHealth
  (return (Variables|/Game/DamageSystem/BPC_DamageSystem.BPC_DamageSystem_C|GetMaxHealth (Variables|Default|GetBPC_DamageSystem))))

(fn GetPatrolRoute
  (return (Variables|Features|GetPatrolRoute)))

(fn Heal
  (params (Amount :type Float%20%28double-precision%29))
  (bind _newhealth (Default|Heal (Variables|Default|GetBPC_DamageSystem) Amount))
  (return _newhealth))

(fn IsDead
  (return (Variables|/Game/DamageSystem/BPC_DamageSystem.BPC_DamageSystem_C|GetIsDead (Variables|Default|GetBPC_DamageSystem))))

(fn SetMovementSpeed
  (params (Speed :type E_MovementSpeed%20Enum :default "NewEnumerator0"))
  (Variables|/Script/Engine.CharacterMovementComponent|SetMaxWalkSpeed (Variables|Character|GetCharacterMovement) (Utilities|Select :Index Speed :NewEnumerator0 0.0 :NewEnumerator1 1.5e+02 :NewEnumerator2 4e+02 :NewEnumerator3 6e+02))
  (return 0.0))

(fn TakeDamage
  (params (DamageInfo :type F%20Damage%20Info%20Structure))
  (bind _wasdamaged (Default|TakeDamage (Variables|Default|GetBPC_DamageSystem) DamageInfo))
  (return _wasdamaged))