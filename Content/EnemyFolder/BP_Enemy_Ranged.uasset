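; Ranged enemy character that spawns a rifle on BeginPlay and attaches it to its hand socket.
; Attack plays a fire montage, whose Fire notify line-traces from the weapon to the AI controller's attack target with debug drawing; the hit result is not yet acted on.
; Montage completion or interruption signals attack end.
; It also maps movement states to walk speeds and supplies fixed attack and defend ranges.
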(event Custom|SpawnWeapon
  (bind _returnvalue (Game|SpawnActorfromClass "/Game/Weapons/BP_WeaponRifle.BP_WeaponRifle_C" (Transformation|GetActorTransform) "Undefined" "MultiplyWithRoot" 0 0))
  (bind _output_get (Variables|Default|SetWeaponActor _returnvalue))
  (Transformation|AttachComponentToComponent _output_get (Variables|Character|GetMesh) "Hand_r_rifle_socket" "SnapToTarget" "SnapToTarget" "SnapToTarget" true)
  (Variables|Default|SetIsWieldingWeapon? true))

(event EventBeginPlay
  (|CallParentFunction)
  (CallFunction|SpawnWeapon))

(event Collision|EventActorBeginOverlap
  (params (OtherActor :type Actor%20Object%20Reference)))

(event EventTick
  (params (DeltaSeconds :type Float%20%28single-precision%29)))

(event EventAttack
  (bind _notifyname (Animation|Montage|PlayMontage (Variables|Character|GetMesh) "/Game/EnemyFolder/Animations/Montage_Rifle_fire.Montage_Rifle_fire")
    (:OnCompleted
      (Default|CallOnAttackEnd :!label _label))
    (:OnInterrupted
      (goto _label))
    (:OnNotifyBegin
      (switch name _notifyname
        (:Fire
          (bind _asaic_enemy_base (Utilities|Casting|CastToAIC_Enemy_Base (AI|GetAIController self)))
          (bind _attacktarget (Variables|/Game/EnemyFolder/AI/AIC_Enemy_Base.AIC_Enemy_Base_C|GetAttackTarget _asaic_enemy_base)
            (:then
              (bind _returnvalue (Collision|LineTraceByChannel (Transformation|GetActorLocation (Variables|Default|GetWeaponActor)) (Transformation|GetActorLocation _attacktarget) "TraceTypeQuery1" false 0 "ForDuration"))
              (if _returnvalue
                _))
            (:else)))))))

(fn ConstructionScript
  (|CallParentFunction))

(fn SetMovementSpeed
  (params (Speed :type E_MovementSpeed%20Enum :default "NewEnumerator0"))
  (Variables|/Script/Engine.CharacterMovementComponent|SetMaxWalkSpeed (Variables|Character|GetCharacterMovement) (Utilities|Select :Index Speed :NewEnumerator0 0.0 :NewEnumerator1 1.7e+02 :NewEnumerator2 4e+02 :NewEnumerator3 6e+02))
  (return 0.0))

(fn GetIdealRange
  (return 5e+02 6e+02))