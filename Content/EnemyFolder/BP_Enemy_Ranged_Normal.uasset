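; Ranged enemy character that spawns a rifle into its hand socket on BeginPlay and fights at long range.
; Attack plays a fire montage whose Fire notify, given a valid AI attack target, launches a projectile from the muzzle aimed at the player character.
; Projectile impact sends damage to the hit actor, and montage completion or interruption signals attack end.
; It also seeds damage-component health, maps movement states to walk speeds and reports its ideal range.
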(event Custom|SpawnWeapon
  (bind _returnvalue (Game|SpawnActorfromClass "/Game/Blueprints/Weapons/BP_WeaponRifle.BP_WeaponRifle_C" (Transformation|GetActorTransform) "Undefined" "MultiplyWithRoot" 0 0))
  (bind _output_get (Variables|Default|SetWeaponVariable _returnvalue))
  (Transformation|AttachComponentToComponent _output_get (Variables|Character|GetMesh) "Hand_r_rifle_socket" "SnapToTarget" "SnapToTarget" "SnapToTarget" true)
  (Variables|Default|SetIsWieldingWeapon? true))

(event Custom|DamagePlayer
  (params (Other%20Actor :type Actor%20Object%20Reference) (Hit :type Hit%20Result%20Structure))
  (Class|BPIDamagable|TakeDamage(Message) Other%20Actor (Utilities|Struct|MakeS_DamageInfo (Variables|EnemyProperties|GetDamageToPlayer) "NewEnumerator1" "NewEnumerator1")))

(event EventBeginPlay
  (|CallParentFunction)
  (CallFunction|SpawnWeapon))

(event Collision|EventActorBeginOverlap
  (params (OtherActor :type Actor%20Object%20Reference)))

(event EventTick
  (params (DeltaSeconds :type Float%20%28single-precision%29)))

(event EventAttack
  (bind _notifyname (Animation|Montage|PlayMontage (Variables|Character|GetMesh) "/Game/EnemyFolder/Animations/Montage_Rifle_fire.Montage_Rifle_fire")
    (:OnCompleted
      (Default|CallOnAttackEnd :!label _label))
    (:OnInterrupted
      (goto _label))
    (:OnNotifyBegin
      (switch name _notifyname
        (:Fire
          (bind _asaic_enemy_base (Utilities|Casting|CastToAIC_Enemy_Base (AI|GetAIController self)))
          (Variables|/Game/EnemyFolder/AI/AIC_Enemy_Base.AIC_Enemy_Base_C|GetAttackTarget _asaic_enemy_base
            (:then
              (bind _returnvalue (Game|SpawnActorfromClass "/Game/Blueprints/BP_Projectile_Rifle.BP_Projectile_Rifle_C" (Transformation|GetWorldTransform (Variables|/Game/Blueprints/Weapons/BP_WeaponRifle.BP_WeaponRifle_C|GetMuzzle (Variables|Default|GetWeaponVariable))) "Undefined" "MultiplyWithRoot" 0 4e+03 0.0 (Game|GetPlayerCharacter 0) false 0))
              (EventDispatchers|BindEventtoOnProjectileImpact _returnvalue (delegate Custom|DamagePlayer)))
            (:else)))))))

(fn ConstructionScript
  (bind _bpc_damagesystem (Variables|Default|GetBPC_DamageSystem))
  (bind _hp (Variables|EnemyProperties|GetHP))
  (|CallParentFunction)
  (Variables|/Game/DamageSystem/BPC_DamageSystem.BPC_DamageSystem_C|SetHealth _bpc_damagesystem _hp)
  (Variables|/Game/DamageSystem/BPC_DamageSystem.BPC_DamageSystem_C|SetMaxHealth _bpc_damagesystem _hp))

(fn SetMovementSpeed
  (params (Speed :type E_MovementSpeed%20Enum :default "NewEnumerator0"))
  (Variables|/Script/Engine.CharacterMovementComponent|SetMaxWalkSpeed (Variables|Character|GetCharacterMovement) (Utilities|Select :Index Speed :NewEnumerator0 0.0 :NewEnumerator1 1.7e+02 :NewEnumerator2 4e+02 :NewEnumerator3 6e+02))
  (return 0.0))

(fn GetIdealRange
  (return 1.4e+03 1.4e+03))