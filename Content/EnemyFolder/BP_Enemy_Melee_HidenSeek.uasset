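; Melee enemy Blueprint that equips a knife and attacks at close range.
; EquipWeapon spawns BP_WeaponKnife on the right-hand socket and flags it as wielded.
; Attack starts a slash montage, immediately sphere-traces forward for pawns to send damage through a struct message, and signals attack end on completion or interruption.
; It supplies attack and defend ranges, while its patrol route and movement speed functions are empty stubs.
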(event EventTick
  (params (DeltaSeconds :type Float%20%28single-precision%29)))

(event Collision|EventActorBeginOverlap
  (params (OtherActor :type Actor%20Object%20Reference)))

(event EventAttack
  (bind _returnvalue (Transformation|GetActorLocation))
  (Animation|Montage|PlayMontage (Variables|Character|GetMesh) "/Game/EnemyFolder/Animations/Montage_Sword_Slash.Montage_Sword_Slash"
    (:then
      (bind (_outhit _returnvalue_2) (Collision|SphereTraceForObjects _returnvalue (+ _returnvalue (* (Math|Vector|GetForwardVector (Transformation|GetActorRotation)) 2e+02)) 2e+01 (Utilities|Array|MakeArray "ObjectTypeQuery3") false 0 "None" true "(R=0.507126,G=0.000000,B=1.000000,A=1.000000)" "(R=0.000000,G=0.456345,B=1.000000,A=1.000000)" 1.0))
      (if _returnvalue_2
        (Class|BPIDamagable|TakeDamage(Message) (.HitActor (Collision|BreakHitResult _outhit)) (Utilities|Struct|MakeS_DamageInfo 1e+01 "NewEnumerator4" "NewEnumerator1"))))
    (:OnCompleted
      (Default|CallOnAttackEnd :!label _label))
    (:OnInterrupted
      (goto _label))))

(event EventEquipWeapon
  (bind _returnvalue (Game|SpawnActorfromClass "/Game/Blueprints/Weapons/BP_WeaponKnife.BP_WeaponKnife_C" (Transformation|GetActorTransform) "Undefined" "MultiplyWithRoot" 0 0))
  (bind _output_get (Variables|Default|SetWeaponActor _returnvalue))
  (Transformation|AttachComponentToComponent _output_get (Variables|Character|GetMesh) "Hand_r_weapon_socket" "SnapToTarget" "SnapToTarget" "SnapToTarget" true)
  (Variables|Default|SetIsWieldingWeapon? true))

(fn ConstructionScript
  (|CallParentFunction))

(fn GetIdealRange
  (return 1.5e+02 6e+02))

(fn GetPatrolRoute
  (return 0))

(fn SetMovementSpeed
  (params (Speed :type E_MovementSpeed%20Enum :default "NewEnumerator0"))
  (return 0.0))