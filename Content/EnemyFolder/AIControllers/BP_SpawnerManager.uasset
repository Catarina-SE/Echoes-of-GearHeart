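; Spawner manager that runs a timed enemy encounter when activated by a keylock, using a "Rerouting Power" countdown.
; Activation starts the spawners through BPI_Activable and two looping timers.
; UpdateTime decrements the time and, at zero, activates end-of-timer targets such as doors.
; CheckTimer refreshes the countdown text each second and, once finished, stops the countdown, shows "System Activated" and deactivates the spawners.
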(event Custom|InitializeCounter
  ;[1 1 1] Initialize Timer and Start Spawning Enemies
  (CallFunction|InitializeTime)
  (bind _returnvalue (Utilities|Time|SetTimerbyFunctionName 0 "UpdateTime" (Variables|TimerOptions|GetTimeDecrementSpeed) true))
  (Variables|TimerOptions|SetSpawnerTimer _returnvalue)
  (CallFunction|ActivateEnemies))

(event Custom|CheckTimer
  (bind _countdowntimer (Variables|Default|GetCountdownTimer))
  ;[1 1 1] Timer Enabled to Check in which step the timer is.
  (Utilities|IsValid _countdowntimer
    (:Is%20Valid
      (Rendering|Components|TextRender|SetText _countdowntimer (Utilities|Text|ToText(String) (Utilities|String|BuildString(Integer) "" "Rerouting Power " (Variables|TimerOptions|GetTime))))
      (Rendering|SetVisibility _countdowntimer true false)
      (if (Variables|TimerOptions|GetbIsFinished)
        (Utilities|Time|ClearandInvalidateTimerbyHandle (Variables|TimerOptions|GetSpawnerTimer))
        (Rendering|Components|TextRender|SetText (Variables|Default|GetCountdownTimer) (Utilities|Text|MakeLiteralText "System Activated"))
        (CallFunction|DeactivateEnemies)))))

(event EventActivate
  (params (Active :type Boolean))
  ;[1 1 1] When Keylock is Activated, Start the Timer And Keep Track of when the timer is finished
  (if Active
    (CallFunction|InitializeCounter)
    (if (Variables|TimerOptions|GetbIsFinished)
      (Utilities|Time|ClearandInvalidateTimerbyHandle (Variables|TimerOptions|GetTimerClockCheckHandler))
      (else
        (bind _returnvalue (Utilities|Time|SetTimerbyFunctionName 0 "CheckTimer" 1.0 true))
        (Variables|TimerOptions|SetTimerClockCheckHandler _returnvalue)))))

(fn ConstructionScript)

(fn UpdateTime
  (bind _endtimeractivables (Variables|Activables|GetEndTimerActivables))
  (Variables|TimerOptions|SetTime (- (Variables|TimerOptions|GetTime) (Variables|TimerOptions|GetTimeDecrementAmount)))
  (if (<= (Variables|TimerOptions|GetTime) 0)
    (Variables|TimerOptions|SetbIsFinished true)
    ;[1 1 1] When Timer is over open the door
    (if (Utilities|Array|IsValidIndex _endtimeractivables)
      (for _array_element _endtimeractivables
        (bind _asbpi_activable (Utilities|Casting|CastToBPI_Activable _array_element))
        (Default|Activate _asbpi_activable true)))))

(fn InitializeTime
  (Variables|TimerOptions|SetTime (Variables|TimerOptions|GetTotalTimerTime)))

(fn StopTime
  (Variables|TimerOptions|SetTime 0))

(fn ActivateEnemies
  (for _array_element (Variables|Activables|GetSpawnersToActivate)
    (bind _asbpi_activable (Utilities|Casting|CastToBPI_Activable _array_element))
    (Default|Activate _asbpi_activable true)))

(fn DeactivateEnemies
  (for _array_element (Variables|Activables|GetSpawnersToActivate)
    (bind _asbpi_activable (Utilities|Casting|CastToBPI_Activable _array_element))
    (Default|Deactivate _asbpi_activable)))