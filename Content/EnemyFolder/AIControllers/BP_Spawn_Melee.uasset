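; BP_Spawn_Melee is a spawner actor that produces melee enemies running the seeker behavior tree.
; Activation spawns one enemy immediately at the Billboard component's location, then repeats on a looping timer set by SpawnRate.
; Deactivation clears and invalidates that timer to stop further spawns.
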(event Custom|InitiateSpawn
  (AI|SpawnAIFromClass (Variables|Default|GetEnemy) "/Game/EnemyFolder/AIControllers/BehaviorTrees/BT_Enemy_Melee_Seeker.BT_Enemy_Melee_Seeker" (Transformation|GetWorldLocation (Variables|Default|GetBillboard)) "0, 0, 0" false 0))

(event EventActivate
  (params (Active :type Boolean))
  (if Active
    (CallFunction|InitiateSpawn)
    (bind _returnvalue (Utilities|Time|SetTimerbyEvent (delegate Custom|InitiateSpawn) (Variables|Default|GetSpawnRate) true))
    (Variables|Default|SetTimer _returnvalue)))

(event EventDeactivate
  (Utilities|Time|ClearandInvalidateTimerbyHandle (Variables|Default|GetTimer)))

(fn ConstructionScript)