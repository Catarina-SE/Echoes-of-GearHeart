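; BP_SpawnerTimer2 is an activated countdown that spawns enemies while power reroutes, then activates a target actor, such as a door.
; Activation shows the countdown text, starts a looping UpdateTime timer and has a BP_AiSpawner2, found by class, spawn immediately and then at SpawnRate until finished.
; At zero, UpdateTime calls BPI_Activable on ActorToActivate.
; Tick refreshes the text, clearing the timer and showing "System Activated" when done.
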(event Custom|InitializeCounter
  ;[1 1 1] Function to Initialize the Timer - Spawn instantly an enemy and then every amount of time spawn new enemies
  (Utilities|FlowControl|Delay 1.0)
  (bind _returnvalue (Actor|GetActorOfClass "/Game/EnemyFolder/AI/BP_AiSpawner2.BP_AiSpawner2_C"))
  (bind _output_get (Variables|Default|SetSpawnerVariable2 _returnvalue))
  (Default|SpawnEnemy _output_get)
  (Rendering|SetVisibility (Variables|Default|GetCountdownTimer) true false)
  (CallFunction|InitializeTime)
  (bind _returnvalue_2 (Utilities|Time|SetTimerbyFunctionName 0 "UpdateTime" (Variables|TimerOptions|GetTimeDecrementSpeed) true))
  (Variables|TimerOptions|SetTimer _returnvalue_2)
  ;;[1 0.2604 0.2604] If the Timer is still running, spawn an enemy every X seconds, if not, stop
  (Utilities|FlowControl|Delay (Variables|TimerOptions|GetSpawnRate) :!label _label)
  (if (not (Variables|Default|GetbIsFinished))
    (Default|SpawnEnemy (Variables|Default|GetSpawnerVariable2))
    (goto _label)))

(event EventActivate
  (params (Active :type Boolean))
  ;[1 1 1] When Keylock is Activated, Start the Timer and open selected door.
  (CallFunction|InitializeCounter))

(event EventTick
  (params (DeltaSeconds :type Float%20%28single-precision%29))
  (bind _countdowntimer (Variables|Default|GetCountdownTimer))
  ;[1 1 1] Tick Enabled to Check in which step the timer is.
  (Utilities|IsValid _countdowntimer
    (:Is%20Valid
      (Rendering|Components|TextRender|SetText _countdowntimer (Utilities|Text|ToText(String) (Utilities|String|BuildString(Integer) "" "Rerouting Power " (Variables|TimerOptions|GetTime))))
      (if (Variables|Default|GetbIsFinished)
        (Utilities|Time|ClearandInvalidateTimerbyHandle (Variables|TimerOptions|GetTimer))
        (Rendering|Components|TextRender|SetText (Variables|Default|GetCountdownTimer) (Utilities|Text|MakeLiteralText "System Activated"))))))

(fn ConstructionScript)

(fn UpdateTime
  (bind _actortoactivate (Variables|ObjectToActivate|GetActorToActivate))
  (Variables|TimerOptions|SetTime (- (Variables|TimerOptions|GetTime) (Variables|TimerOptions|GetTimeDecrementAmount)))
  (if (<= (Variables|TimerOptions|GetTime) 0)
    ;[1 1 1] When Timer is over open the door
    (Variables|Default|SetbIsFinished true)
    (Utilities|IsValid _actortoactivate
      (:Is%20Valid
        (bind _asbpi_activable (Utilities|Casting|CastToBPI_Activable _actortoactivate))
        (Default|Activate _asbpi_activable true)))))

(fn InitializeTime
  (Variables|TimerOptions|SetTime (Variables|TimerOptions|GetMaxTime)))

(fn StopTime
  (Variables|TimerOptions|SetTime 0))