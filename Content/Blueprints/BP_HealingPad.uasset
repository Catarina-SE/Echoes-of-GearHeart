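; BP_HealingPad is an interactable pad that heals the player on an IA_Interact press.
; Box overlap toggles input on the pad and shows or hides a prompt widget.
; Interacting at max health shows a warning widget for three seconds.
; Otherwise it calls the player's Heal function, plays a syringe sound, stops the low-health audio and re-arms that sound's trigger flag.
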(event OnComponentBeginOverlap(Box)
  (params (OverlappedComponent :type Primitive%20Component%20Object%20Reference) (OtherActor :type Actor%20Object%20Reference) (OtherComp :type Primitive%20Component%20Object%20Reference) (OtherBodyIndex :type Integer) (bFromSweep :type Boolean) (SweepResult :type Hit%20Result%20Structure%20%28by%20ref%29))
  ;[1 1 1] Enabling/Disabling Input
  (Input|EnableInput (Game|GetPlayerController 0))
  (Rendering|SetVisibility (Variables|Default|GetWidget) true false))

(event OnComponentEndOverlap(Box)
  (params (OverlappedComponent :type Primitive%20Component%20Object%20Reference) (OtherActor :type Actor%20Object%20Reference) (OtherComp :type Primitive%20Component%20Object%20Reference) (OtherBodyIndex :type Integer))
  ;[1 1 1] Enabling/Disabling Input
  (Input|DisableInput (Game|GetPlayerController 0))
  (Rendering|SetVisibility (Variables|Default|GetWidget) false false))

(event Input|EnhancedActionEvents|EnhancedInputActionIA_Interact
  (params (ActionValue :type Boolean) (ElapsedSeconds :type Float%20%28double-precision%29) (TriggeredSeconds :type Float%20%28double-precision%29) (InputAction :type Input%20Action%20Object%20Reference :default "/Game/PlayerFolder/Input/Actions/IA_Interact.IA_Interact"))
  (bind _maxhealthwarning (Variables|Default|GetMaxHealthWarning))
  ;[1 1 1] On Interact if health is full show warning message, if its not full cast to the player and activate its healing function
  (:Started
    (bind _asbp_player (Utilities|Casting|CastToBP_Player (Game|Player|GetPlayerPawn 0)))
    (bind _output_get (Variables|Default|SetPlayerReference _asbp_player))
    (if (== (Variables|/Game/DamageSystem/BPC_DamageSystem.BPC_DamageSystem_C|GetHealth (Variables|/Game/PlayerFolder/Blueprints/BP_Player.BP_Player_C|GetBPC_DamageSystem _output_get)) (Variables|/Game/DamageSystem/BPC_DamageSystem.BPC_DamageSystem_C|GetMaxHealth (Variables|/Game/PlayerFolder/Blueprints/BP_Player.BP_Player_C|GetBPC_DamageSystem _output_get)))
      (Rendering|SetVisibility _maxhealthwarning true false)
      (Utilities|FlowControl|Delay 3.0)
      (Rendering|SetVisibility _maxhealthwarning false false)
      (else
        (Default|Heal _output_get (Variables|Default|GetHealing%20Stat))
        (Audio|PlaySound2D "/Game/Audio/SyringeHealing.SyringeHealing" 1.0 1.0 0.0 0 0)
        ;;[1 0.2829 0] Resets Variable so that next time the sound trigger can execute again
        (Variables|/Game/PlayerFolder/Blueprints/BP_Player.BP_Player_C|SetCanPlaySound (Variables|Default|GetPlayerReference) true)
        (Audio|Components|Audio|Stop (Variables|/Game/PlayerFolder/Blueprints/BP_Player.BP_Player_C|GetLowHealthAudioReference (Variables|Default|GetPlayerReference)))))))

(fn ConstructionScript)