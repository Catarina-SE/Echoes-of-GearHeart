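; BP_SimpleKeylock is an interactable keylock that activates a linked actor, such as a door.
; Player overlap with its box shows a prompt widget and enables input for IA_Interact.
; Interacting first steps through any DialogSequence via BP_GameMode, opening once dialogue ends; without dialogue it opens immediately.
; Opening calls Activate through BPI_Activable, disables input on the player controller, turns the mesh green and plays a click.
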(event OnComponentBeginOverlap(Box)
  (params (OverlappedComponent :type Primitive%20Component%20Object%20Reference) (OtherActor :type Actor%20Object%20Reference) (OtherComp :type Primitive%20Component%20Object%20Reference) (OtherBodyIndex :type Integer) (bFromSweep :type Boolean) (SweepResult :type Hit%20Result%20Structure%20%28by%20ref%29))
  (Utilities|Casting|CastToBP_Player OtherActor)
  (Input|EnableInput (Game|GetPlayerController 0))
  (Rendering|SetVisibility (Variables|Default|GetWidget) true false))

(event OnComponentEndOverlap(Box)
  (params (OverlappedComponent :type Primitive%20Component%20Object%20Reference) (OtherActor :type Actor%20Object%20Reference) (OtherComp :type Primitive%20Component%20Object%20Reference) (OtherBodyIndex :type Integer))
  (Utilities|Casting|CastToBP_Player OtherActor)
  (Rendering|SetVisibility (Variables|Default|GetWidget) false false))

(event Input|EnhancedActionEvents|EnhancedInputActionIA_Interact
  (params (ActionValue :type Boolean) (ElapsedSeconds :type Float%20%28double-precision%29) (TriggeredSeconds :type Float%20%28double-precision%29) (InputAction :type Input%20Action%20Object%20Reference :default "/Game/PlayerFolder/Input/Actions/IA_Interact.IA_Interact"))
  ;[1 1 1] IF door is not open Open it
  (:Started
    (if (Utilities|Array|IsValidIndex (Variables|Default|GetDialogSequence))
      (if (Variables|Default|GetHasStartedDialog)
        (Default|ShowNextDialogue (Variables|Default|GetGameModeVariable))
        (else
          (Variables|Default|SetHasStartedDialog true)
          (Variables|/Game/Blueprints/BP_GameMode.BP_GameMode_C|SetEndofDialogue (Variables|Default|GetGameModeVariable) false)
          (Default|StartDialogue (Variables|Default|GetGameModeVariable) (Variables|Default|GetDialogSequence))))
      (else
        (CallFunction|OpenDoor))))
  (:Completed
    (if (Variables|/Game/Blueprints/BP_GameMode.BP_GameMode_C|GetEndofDialogue (Variables|Default|GetGameModeVariable))
      (CallFunction|OpenDoor))))

(event EventBeginPlay
  (bind _asbp_game_mode (Utilities|Casting|CastToBP_GameMode (Game|GetGameMode)))
  (Variables|Default|SetGameModeVariable _asbp_game_mode))

(fn ConstructionScript)

(fn OpenDoor
  (Utilities|ActivateDoor true)
  (Input|DisableInput (Game|GetPlayerController 0) 0)
  (Rendering|Material|SetMaterial (Variables|Default|GetKeylock%20Mesh) 0 "/Game/Level_Art/MI_Light_Green.MI_Light_Green")
  (Audio|PlaySound2D "/Engine/VREditor/Sounds/UI/Click_on_Button_Cue.Click_on_Button_Cue" 1.0 1.0 0.0 0 0))