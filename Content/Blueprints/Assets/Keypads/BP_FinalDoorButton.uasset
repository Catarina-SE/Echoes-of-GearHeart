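; BP_FinalDoorButton is a keypad button, named for the final door, that starts out locked.
; On BeginPlay it runs the parent logic, clears CanBeInteracted, disables Box collision and sets an orange light material on KeyLockBig.
; An Activate event with a true value switches Box to query-only collision, leaving CanBeInteracted and the material untouched.
; The graph holds no press or door-opening logic of its own.
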(event EventBeginPlay
  (|CallParentFunction)
  (Variables|Default|SetbCanBeInteracted false)
  (Collision|SetCollisionEnabled (Variables|Default|GetBox) "NoCollision")
  (Rendering|Material|SetMaterial (Variables|Default|GetKeyLockBig) 1 "/Game/Level_Art/MI_Light_Orange.MI_Light_Orange"))

(event Collision|EventActorBeginOverlap
  (params (OtherActor :type Actor%20Object%20Reference)))

(event EventTick
  (params (DeltaSeconds :type Float%20%28single-precision%29)))

(event EventActivate
  (params (Active :type Boolean))
  (if Active
    (Collision|SetCollisionEnabled (Variables|Default|GetBox) "QueryOnly")))

(fn ConstructionScript
  (|CallParentFunction))