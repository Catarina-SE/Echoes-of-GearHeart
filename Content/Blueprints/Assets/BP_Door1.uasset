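; Door Blueprint that slides its Door component along local Z when switched by the Activate event.
; Activate plays DoorTimeline at a rate set by TimetoOpen or reverses it; every update lerps the position and sets IsDoorOpen true, even while closing.
; A player leaving Collision reverses a separate Timeline, never played forward here, that drives the same offset.
; Despite their DoorRotationZ name, both tracks drive translation.
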(event OnComponentEndOverlap(Collision)
  (params (OverlappedComponent :type Primitive%20Component%20Object%20Reference) (OtherActor :type Actor%20Object%20Reference) (OtherComp :type Primitive%20Component%20Object%20Reference) (OtherBodyIndex :type Integer))
  (Utilities|Casting|CastToBP_Player OtherActor)
  (bind _doorrotationz (Timeline|Timeline Reverse)
    (:Update
      (Transformation|SetRelativeLocation (Variables|Default|GetDoor) (Math|Vector|Lerp(Vector) "0, 0, 0" "0.000000,0.000000,2.700000" _doorrotationz) false false))))

(event EventBeginPlay)

(event Collision|EventActorBeginOverlap
  (params (OtherActor :type Actor%20Object%20Reference)))

(event EventTick
  (params (DeltaSeconds :type Float%20%28single-precision%29)))

(event EventActivate
  (params (Active :type Boolean))
  (if Active
    (Components|Timeline|SetPlayRate (Variables|Default|GetDoorTimeline) (/ 1.0 (Variables|Default|GetTimetoOpen)))
    (bind _doorrotationz (Timeline|DoorTimeline Play)
      (:Update
        (Transformation|SetRelativeLocation (Variables|Default|GetDoor) (Math|Vector|Lerp(Vector) "0, 0, 0" "0.000000,0.000000,2.700000" _doorrotationz) false false)
        (Variables|Default|SetbIsDoorOpen true)))
    (else
      (Timeline|DoorTimeline Reverse))))

(fn ConstructionScript)