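; BP_SimpleKeylock is a one-shot interaction trigger that activates a referenced actor, such as a door.
; The first overlap with its Box passes a DoOnce and enables input on the lock.
; IA_Interact then calls ActivateDoor, which sends Activate to ActorToActivate through BPI_Activable, then calls DisableInput.
; ActivateDoor prints a warning if the target lacks that interface.
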(event OnComponentBeginOverlap(Box)
  (params (OverlappedComponent :type Primitive%20Component%20Object%20Reference) (OtherActor :type Actor%20Object%20Reference) (OtherComp :type Primitive%20Component%20Object%20Reference) (OtherBodyIndex :type Integer) (bFromSweep :type Boolean) (SweepResult :type Hit%20Result%20Structure%20%28by%20ref%29))
  (Utilities|FlowControl|DoOnce false
    (:Completed
      (Input|EnableInput (Game|GetPlayerController 0)))))

(event Input|EnhancedActionEvents|EnhancedInputActionIA_Interact
  (params (ActionValue :type Boolean) (ElapsedSeconds :type Float%20%28double-precision%29) (TriggeredSeconds :type Float%20%28double-precision%29) (InputAction :type Input%20Action%20Object%20Reference :default "/Game/PlayerFolder/Input/Actions/IA_Interact.IA_Interact"))
  ;[1 1 1] IF door is not open Open it
  (Utilities|ActivateDoor true)
  (Input|DisableInput (Game|GetPlayerController 0) 0))

(event EventBeginPlay
  (bind _asbp_player (Utilities|Casting|CastToBP_Player (Game|GetPlayerCharacter 0)))
  (Variables|Default|SetPlayerReference _asbp_player))

(fn ConstructionScript)