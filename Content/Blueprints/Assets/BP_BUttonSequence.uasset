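; Arrow-key sequence puzzle that opens a door or other linked BPI_Activable actor.
; The Box overlap gates input, and IA_Interact hides the player mesh and weapon, disables pawn input if unsolved, and blends to a static camera.
; Arrow presses are checked against UnlockSequence, with a wrong key resetting the index.
; Completing the sequence activates the linked actor and restores player visibility, input and view.
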(event OnComponentBeginOverlap(Box)
  (params (OverlappedComponent :type Primitive%20Component%20Object%20Reference) (OtherActor :type Actor%20Object%20Reference) (OtherComp :type Primitive%20Component%20Object%20Reference) (OtherBodyIndex :type Integer) (bFromSweep :type Boolean) (SweepResult :type Hit%20Result%20Structure%20%28by%20ref%29))
  (Input|EnableInput (Game|GetPlayerController 0)))

(event OnComponentEndOverlap(Box)
  (params (OverlappedComponent :type Primitive%20Component%20Object%20Reference) (OtherActor :type Actor%20Object%20Reference) (OtherComp :type Primitive%20Component%20Object%20Reference) (OtherBodyIndex :type Integer))
  (Input|DisableInput (Game|GetPlayerController 0)))

(event Input|EnhancedActionEvents|EnhancedInputActionIA_Interact
  (params (ActionValue :type Boolean) (ElapsedSeconds :type Float%20%28double-precision%29) (TriggeredSeconds :type Float%20%28double-precision%29) (InputAction :type Input%20Action%20Object%20Reference :default "/Game/PlayerFolder/Input/Actions/IA_Interact.IA_Interact"))
  (bind _playerreference (Variables|Default|GetPlayerReference))
  (Rendering|SetVisibility (Variables|/Script/Engine.Character|GetMesh _playerreference) false false)
  (Rendering|SetVisibility (Variables|/Game/PlayerFolder/Blueprints/BP_Player.BP_Player_C|GetBP_Weapon_Base _playerreference) false false)
  (if (not (Variables|Default|GetbIsDoorOpen))
    ;[1 1 1] IF door is not open Open it
    (Utilities|ToggleCharacterMovement false
      (:Out
        (Utilities|ChangeViewStaticCamera)))))

(event EventBeginPlay
  (bind _asbp_player (Utilities|Casting|CastToBP_Player (Game|GetPlayerCharacter 0)))
  (Variables|Default|SetPlayerReference _asbp_player))

(event Input|KeyboardEvents|Down
  (params (Key :type Key%20Structure :default "None"))
  (:Pressed
    (if (== (Utilities|Array|Get(acopy) (Variables|Default|GetUnlockSequence) (Variables|Default|GetIndex)) 2)
      (CallFunction|IsSequenceCompleted)
      (else
        (Variables|Default|SetIndex 0)))))

(event Input|KeyboardEvents|Up
  (params (Key :type Key%20Structure :default "None"))
  ;[0 0.1634 1] Returns the item in the array at the index -> sets it to 1 (Up Key)
  (:Pressed
    (if (== (Utilities|Array|Get(acopy) (Variables|Default|GetUnlockSequence) (Variables|Default|GetIndex)) 1)
      (CallFunction|IsSequenceCompleted)
      (else
        (Variables|Default|SetIndex 0)))))

(event Input|KeyboardEvents|Right
  (params (Key :type Key%20Structure :default "None"))
  (:Pressed
    (if (== (Utilities|Array|Get(acopy) (Variables|Default|GetUnlockSequence) (Variables|Default|GetIndex)) 4)
      (CallFunction|IsSequenceCompleted)
      (else
        (Variables|Default|SetIndex 0)))))

(event Input|KeyboardEvents|Left
  (params (Key :type Key%20Structure :default "None"))
  (:Pressed
    (if (== (Utilities|Array|Get(acopy) (Variables|Default|GetUnlockSequence) (Variables|Default|GetIndex)) 3)
      (CallFunction|IsSequenceCompleted)
      (else
        (Variables|Default|SetIndex 0)))))

(fn ConstructionScript)

(fn ResetSequence)

(fn IsSequenceCompleted
  (bind _playerreference (Variables|Default|GetPlayerReference))
  (if (== (- (Utilities|Array|Length (Variables|Default|GetUnlockSequence)) 1) (Variables|Default|GetIndex))
    (Variables|Default|SetbIsDoorOpen true)
    (Utilities|ActivateDoor true)
    (Rendering|SetVisibility (Variables|/Script/Engine.Character|GetMesh _playerreference) true false)
    (Rendering|SetVisibility (Variables|/Game/PlayerFolder/Blueprints/BP_Player.BP_Player_C|GetBP_Weapon_Base _playerreference) true false)
    (Utilities|ToggleCharacterMovement true
      (:Out
        (Utilities|ChangeViewtoControllerCamera)))
    (else
      (Math|Integer|IncrementInt (Variables|Default|GetIndex)))))