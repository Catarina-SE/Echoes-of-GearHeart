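; BP_Radio is an interactable radio that plays a dialogue sequence and then activates a linked actor.
; Its Box overlap toggles input, so IA_Interact starts or advances the dialogue through BP_GameMode.
; When the interact input completes after dialogue ends, ActivateDoor switches on ActorToActivate through BPI_Activable and calls DisableInput.
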(event OnComponentBeginOverlap(Box)
  (params (OverlappedComponent :type Primitive%20Component%20Object%20Reference) (OtherActor :type Actor%20Object%20Reference) (OtherComp :type Primitive%20Component%20Object%20Reference) (OtherBodyIndex :type Integer) (bFromSweep :type Boolean) (SweepResult :type Hit%20Result%20Structure%20%28by%20ref%29))
  (Input|EnableInput (Game|GetPlayerController 0)))

(event OnComponentEndOverlap(Box)
  (params (OverlappedComponent :type Primitive%20Component%20Object%20Reference) (OtherActor :type Actor%20Object%20Reference) (OtherComp :type Primitive%20Component%20Object%20Reference) (OtherBodyIndex :type Integer))
  (Input|DisableInput (Game|GetPlayerController 0)))

(event Input|EnhancedActionEvents|EnhancedInputActionIA_Interact
  (params (ActionValue :type Boolean) (ElapsedSeconds :type Float%20%28double-precision%29) (TriggeredSeconds :type Float%20%28double-precision%29) (InputAction :type Input%20Action%20Object%20Reference :default "/Game/PlayerFolder/Input/Actions/IA_Interact.IA_Interact"))
  (:Started
    (if (Variables|Default|GetHasStartedDialogue)
      (Default|ShowNextDialogue (Variables|Default|GetGameModeVariable))
      (else
        (Variables|Default|SetHasStartedDialogue true)
        (Default|StartDialogue (Variables|Default|GetGameModeVariable) (Variables|Default|GetDialogueSequence)))))
  (:Completed
    (if (Variables|/Game/Blueprints/BP_GameMode.BP_GameMode_C|GetEndofDialogue (Variables|Default|GetGameModeVariable))
      (Utilities|IsValid (Variables|Default|GetActorToActivate)
        (:Is%20Valid
          (Utilities|ActivateDoor true))))))

(event Collision|EventActorBeginOverlap
  (params (OtherActor :type Actor%20Object%20Reference)))

(event EventTick
  (params (DeltaSeconds :type Float%20%28single-precision%29)))

(event EventBeginPlay
  (bind _asbp_game_mode (Utilities|Casting|CastToBP_GameMode (Game|GetGameMode))
    (:then
      (Variables|Default|SetGameModeVariable _asbp_game_mode))
    (:CastFailed
      (Development|PrintString "CastFailed"))))

(fn ConstructionScript)