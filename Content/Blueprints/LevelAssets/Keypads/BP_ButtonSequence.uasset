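; Keypad lock puzzle where the player enters an arrow-key sequence to activate a linked actor, such as a door.
; Box overlap enables input; interacting hides player and weapon, disables movement and switches to a static camera.
; Arrow presses are checked against UnlockSequence, lighting correct arrows green or resetting with an error.
; Completion calls BPI_Activable and restores the player; construction flags choose small or big keypad meshes.
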(event OnComponentBeginOverlap(Box)
  (params (OverlappedComponent :type Primitive%20Component%20Object%20Reference) (OtherActor :type Actor%20Object%20Reference) (OtherComp :type Primitive%20Component%20Object%20Reference) (OtherBodyIndex :type Integer) (bFromSweep :type Boolean) (SweepResult :type Hit%20Result%20Structure%20%28by%20ref%29))
  (Input|EnableInput (Game|GetPlayerController 0))
  (Rendering|SetVisibility (Variables|Default|GetInteractionHint) true false))

(event OnComponentEndOverlap(Box)
  (params (OverlappedComponent :type Primitive%20Component%20Object%20Reference) (OtherActor :type Actor%20Object%20Reference) (OtherComp :type Primitive%20Component%20Object%20Reference) (OtherBodyIndex :type Integer))
  (Input|DisableInput (Game|GetPlayerController 0))
  (Rendering|SetVisibility (Variables|Default|GetInteractionHint) false false))

(event Input|EnhancedActionEvents|EnhancedInputActionIA_Interact
  (params (ActionValue :type Boolean) (ElapsedSeconds :type Float%20%28double-precision%29) (TriggeredSeconds :type Float%20%28double-precision%29) (InputAction :type Input%20Action%20Object%20Reference :default "/Game/Blueprints/PlayerFolder/Input/Actions/IA_Interact.IA_Interact"))
  (bind _playerreference (Variables|Default|GetPlayerReference))
  ;[1 1 1] IF door is not open Open it
  (Rendering|SetVisibility (Variables|/Script/Engine.Character|GetMesh _playerreference) false false)
  (Rendering|SetVisibility (Variables|/Game/Blueprints/PlayerFolder/Blueprints/BP_Player.BP_Player_C|GetBP_Weapon_Base _playerreference) false false)
  (if (not (Variables|Default|GetbIsDoorOpen))
    (Utilities|ToggleCharacterMovement false
      (:Out
        (Utilities|ChangeViewStaticCamera)))))

(event EventBeginPlay
  (bind _asbp_player (Utilities|Casting|CastToBP_Player (Game|GetPlayerCharacter 0)))
  (Variables|Default|SetPlayerReference _asbp_player))

(event Input|KeyboardEvents|Down
  (params (Key :type Key%20Structure))
  ;[0.1354 0.1354 0.1354] CodeLock Logic
  (:Pressed
    (if (== (Utilities|Array|Get(acopy) (Variables|Default|GetUnlockSequence) (Variables|Default|GetIndex)) 2)
      (CallFunction|IsSequenceCompleted)
      (Rendering|Material|SetMaterial (Variables|Default|GetDOWN) 0 "/AnimationSharing/AnimSharingGreen.AnimSharingGreen")
      (Audio|PlaySound2D "/Engine/VREditor/Sounds/UI/Selection_Changes.Selection_Changes" 1.0 1.0 0.0 0 0)
      (else
        (Variables|Default|SetIndex 0)
        (Audio|PlaySound2D (Variables|Default|GetSoundWhenIncorrect) 1.0 1.0 0.0 0 0)
        (CallFunction|ResetColors)
        (Utilities|ToggleErrorMessage)))))

(event Input|KeyboardEvents|Up
  (params (Key :type Key%20Structure))
  ;[0.1354 0.1354 0.1354] CodeLock Logic
  ;;[0 0.1634 1] Returns the item in the array at the index -> sets it to 1 (Up Key)
  (:Pressed
    (if (== (Utilities|Array|Get(acopy) (Variables|Default|GetUnlockSequence) (Variables|Default|GetIndex)) 1)
      (CallFunction|IsSequenceCompleted)
      (Rendering|Material|SetMaterial (Variables|Default|GetUP) 0 "/AnimationSharing/AnimSharingGreen.AnimSharingGreen")
      (Audio|PlaySound2D "/Engine/VREditor/Sounds/UI/Selection_Changes.Selection_Changes" 1.0 1.0 0.0 0 0)
      (else
        ;;[1 1 1] Logic When Input is Incorrect
        (Variables|Default|SetIndex 0)
        (Audio|PlaySound2D (Variables|Default|GetSoundWhenIncorrect) 1.0 1.0 0.0 0 0)
        (CallFunction|ResetColors)
        (Utilities|ToggleErrorMessage)))))

(event Input|KeyboardEvents|Right
  (params (Key :type Key%20Structure))
  ;[0.1354 0.1354 0.1354] CodeLock Logic
  (:Pressed
    (if (== (Utilities|Array|Get(acopy) (Variables|Default|GetUnlockSequence) (Variables|Default|GetIndex)) 4)
      (CallFunction|IsSequenceCompleted)
      (Rendering|Material|SetMaterial (Variables|Default|GetRIGHT) 0 "/AnimationSharing/AnimSharingGreen.AnimSharingGreen")
      (Audio|PlaySound2D "/Engine/VREditor/Sounds/UI/Selection_Changes.Selection_Changes" 1.0 1.0 0.0 0 0)
      (else
        (Variables|Default|SetIndex 0)
        (Audio|PlaySound2D (Variables|Default|GetSoundWhenIncorrect) 1.0 1.0 0.0 0 0)
        (CallFunction|ResetColors)
        (Utilities|ToggleErrorMessage)))))

(event Input|KeyboardEvents|Left
  (params (Key :type Key%20Structure))
  ;[0.1354 0.1354 0.1354] CodeLock Logic
  (:Pressed
    (if (== (Utilities|Array|Get(acopy) (Variables|Default|GetUnlockSequence) (Variables|Default|GetIndex)) 3)
      (CallFunction|IsSequenceCompleted)
      (Rendering|Material|SetMaterial (Variables|Default|GetLEFT) 0 "/AnimationSharing/AnimSharingGreen.AnimSharingGreen")
      (Audio|PlaySound2D "/Engine/VREditor/Sounds/UI/Selection_Changes.Selection_Changes" 1.0 1.0 0.0 0 0)
      (else
        (Variables|Default|SetIndex 0)
        (Audio|PlaySound2D (Variables|Default|GetSoundWhenIncorrect) 1.0 1.0 0.0 0 0)
        (CallFunction|ResetColors)
        (Utilities|ToggleErrorMessage)))))

(fn ConstructionScript
  (bind _keylocksmall (Variables|Default|GetKeyLockSmall))
  (bind _keylockbig (Variables|Default|GetKeyLockBig))
  (Utilities|FlowControl|Sequence
    (:then_0
      (if (Variables|Default|GetKeyPadSmall)
        (Rendering|SetVisibility _keylocksmall true false)
        (else
          (Rendering|SetVisibility _keylocksmall false false))))
    (:then_1
      (if (Variables|Default|GetKeyPadBig)
        (Rendering|SetVisibility _keylockbig true false)
        (else
          (Rendering|SetVisibility _keylockbig false false))))))

(fn ResetSequence)

(fn IsSequenceCompleted
  (bind _playerreference (Variables|Default|GetPlayerReference))
  (if (== (- (Utilities|Array|Length (Variables|Default|GetUnlockSequence)) 1) (Variables|Default|GetIndex))
    (Variables|Default|SetbIsDoorOpen true)
    (Utilities|ActivateDoor true)
    (Rendering|SetVisibility (Variables|/Script/Engine.Character|GetMesh _playerreference) true false)
    (Rendering|SetVisibility (Variables|/Game/Blueprints/PlayerFolder/Blueprints/BP_Player.BP_Player_C|GetBP_Weapon_Base _playerreference) true false)
    (Utilities|ToggleCharacterMovement true
      (:Out
        (Utilities|ChangeViewtoControllerCamera)
        (if (Variables|Default|GetKeyPadSmall)
          (Rendering|Material|SetMaterial (Variables|Default|GetKeyLockSmall) 0 "/Game/Level_Art/MI_Light_Green.MI_Light_Green")
          (Audio|PlaySound2D "/Engine/VREditor/Sounds/UI/Click_on_Button_Cue.Click_on_Button_Cue" 1.0 1.0 0.0 0 0 :!label _label)
          (elif (Variables|Default|GetKeyPadBig)
            (Rendering|Material|SetMaterial (Variables|Default|GetKeyLockBig) 1 "/Game/Level_Art/MI_Light_Green.MI_Light_Green")
            (goto _label)))))
    (else
      (Math|Integer|IncrementInt (Variables|Default|GetIndex)))))

(fn ResetColors
  (Rendering|Material|SetMaterial (Variables|Default|GetRIGHT) 0 "/Game/Level_Art/Arrow_Rubber.Arrow_Rubber"))