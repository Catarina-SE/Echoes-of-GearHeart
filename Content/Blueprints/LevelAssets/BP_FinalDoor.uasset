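; BP_FinalDoor is the level's final door, which opens on activation and brings up the end menu.
; Activate runs a timeline, rate-scaled by TimetoOpen, that lerps the door mesh along Z and sets IsDoorOpen to block reactivation.
; Any overlap with the Collision component, with no actor filter or open-state check, shows WBP_EndMenu, pauses the game and reveals the mouse cursor.
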(event OnComponentBeginOverlap(Collision)
  (params (OverlappedComponent :type Primitive%20Component%20Object%20Reference) (OtherActor :type Actor%20Object%20Reference) (OtherComp :type Primitive%20Component%20Object%20Reference) (OtherBodyIndex :type Integer) (bFromSweep :type Boolean) (SweepResult :type Hit%20Result%20Structure%20%28by%20ref%29))
  ;[1 0 0.01854] Prevention to not allow enemies to close doors
  (bind _returnvalue (UserInterface|CreateWidget "/Game/Blueprints/Widgets/WBP_EndMenu.WBP_EndMenu_C"))
  (UserInterface|Viewport|AddtoViewport _returnvalue 0)
  (Game|SetGamePaused true)
  (Variables|/Script/Engine.PlayerController|SetbShowMouseCursor (Game|GetPlayerController 0) true))

(event EventBeginPlay)

(event Collision|EventActorBeginOverlap
  (params (OtherActor :type Actor%20Object%20Reference)))

(event EventTick
  (params (DeltaSeconds :type Float%20%28single-precision%29)))

(event EventActivate
  (params (Active :type Boolean))
  (if (not (Variables|Default|GetbIsDoorOpen))
    (Components|Timeline|SetPlayRate (Variables|Default|GetDoorTimeline) (/ 1.0 (Variables|Default|GetTimetoOpen)))
    (bind _doorrotationz (Timeline|DoorTimeline Play)
      (:Update
        (Transformation|SetRelativeLocation (Variables|Default|GetDoor) (Math|Vector|Lerp(Vector) "0, 0, 0" "0.000000,0.000000,3.000000" _doorrotationz) false false)
        (Variables|Default|SetbIsDoorOpen true)))))

(fn ConstructionScript)