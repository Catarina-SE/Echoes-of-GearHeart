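; BP_GameMode is a game mode Blueprint that provides helper functions for the player's UI.
; ToggleMenu opens the in-game menu, pausing the game and switching input to UI only with a visible cursor, but has no closing branch.
; Crosshair functions add or remove a stored aim widget, and ActivateHealthBar creates a health widget bound to BP_Player.
; ActivateTimer is an empty stub with disconnected countdown logic, and Tick sets a timer with no event.
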(event EventBeginPlay)

(event EventTick
  (params (DeltaSeconds :type Float%20%28single-precision%29))
  (Utilities|Time|SetTimerbyEvent 0 0.0))

(fn ConstructionScript)

(fn ToggleMenu
  (bind _returnvalue (Game|GetPlayerController 0))
  (bind _returnvalue_2 (UserInterface|CreateWidget "/Game/Blueprints/Widgets/WBP_InGameMenu.WBP_InGameMenu_C"))
  (UserInterface|Viewport|AddtoViewport _returnvalue_2 0)
  (Variables|/Script/Engine.PlayerController|SetbShowMouseCursor _returnvalue true)
  (Input|SetInputModeUIOnly _returnvalue 0 "DoNotLock" false)
  (Game|SetGamePaused true))

(fn EnableCrossHair
  (bind _returnvalue (UserInterface|CreateWidget "/Game/Blueprints/Widgets/WBP_PlayerAim.WBP_PlayerAim_C"))
  (bind _output_get (Variables|Default|SetCrossHairReference _returnvalue))
  (UserInterface|Viewport|AddtoViewport _output_get 0))

(fn DisableCrossHair
  (Widget|RemovefromParent (Variables|Default|GetCrossHairReference)))

(fn ActivateHealthBar
  (bind _asbp_player (Utilities|Casting|CastToBP_Player (Game|Player|GetPlayerPawn 0)))
  (bind _output_get (Variables|Default|SetAs%20BP%20Player _asbp_player))
  (bind _returnvalue (UserInterface|CreateWidget "/Game/DamageSystem/WBP_PlayerHealth.WBP_PlayerHealth_C" 0 _output_get))
  (UserInterface|Viewport|AddtoViewport _returnvalue 0))

(fn ActivateTimer)