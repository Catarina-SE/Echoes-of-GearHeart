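; Base projectile actor for weapons, with configurable speed, gravity and an optional target.
; The construction script configures ProjectileMovement and enables homing on the target's root component when IsHoming is set.
; On BeginPlay, a valid target redirects velocity straight toward it.
; A box collision hit fires the OnProjectileImpact dispatcher, spawns impact effect and sound, destroys the actor and updates the player's SpawnedBullets list.
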(event OnComponentHit(BoxCollision)
  (params (HitComponent :type Primitive%20Component%20Object%20Reference) (OtherActor :type Actor%20Object%20Reference) (OtherComp :type Primitive%20Component%20Object%20Reference) (NormalImpulse :type Vector :default "0, 0, 0") (Hit :type Hit%20Result%20Structure%20%28by%20ref%29))
  (bind _location (Collision|BreakHitResult Hit))
  (Default|CallOnProjectileImpact OtherActor Hit)
  (Effects|SpawnEmitteratLocation (Variables|Default|GetImpactEffect) _location)
  (Audio|PlaySoundatLocation (Variables|Default|GetImpactSound) _location "0, 0, 0" 1.0 1.0 0.0 0 0 0 0)
  (Actor|DestroyActor)
  (bind _asbp_player (Utilities|Casting|CastToBP_Player (Game|GetPlayerCharacter 0)))
  (Utilities|Array|RemoveItem (Variables|/Game/Blueprints/PlayerFolder/Blueprints/BP_Player.BP_Player_C|GetSpawnedBullets _asbp_player) 0))

(event Custom|FocusTarget
  (Variables|/Script/Engine.MovementComponent|SetVelocity (Variables|Default|GetProjectileMovement) (* (Math|Vector|GetUnitDirection(Vector) (Transformation|GetActorLocation) (Transformation|GetActorLocation (Variables|Default|GetTarget))) (Variables|ProjectileSettings|GetSpeed))))

(event EventBeginPlay
  (Variables|Default|GetTarget
    (:then
      (CallFunction|FocusTarget))
    (:else)))

(fn ConstructionScript
  (bind _projectilemovement (Variables|Default|GetProjectileMovement))
  (bind _speed (Variables|ProjectileSettings|GetSpeed))
  (Variables|/Script/Engine.ProjectileMovementComponent|SetInitialSpeed _projectilemovement _speed)
  (Variables|/Script/Engine.ProjectileMovementComponent|SetMaxSpeed _projectilemovement _speed)
  (Variables|/Script/Engine.ProjectileMovementComponent|SetProjectileGravityScale _projectilemovement (Variables|ProjectileSettings|GetGravity))
  (Variables|Default|GetTarget
    (:then
      (if (Variables|Default|GetisHoming)
        (Variables|/Script/Engine.ProjectileMovementComponent|SetbIsHomingProjectile _projectilemovement true)
        (Variables|/Script/Engine.ProjectileMovementComponent|SetHomingTargetComponent _projectilemovement (Variables|/Script/Engine.Actor|GetRootComponent (Variables|Default|GetTarget)))))
    (:else)))