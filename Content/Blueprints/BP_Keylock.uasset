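; BP_Keylock is an interactable switch that opens and closes a linked door while the player stands in its trigger box.
; Box overlap enables or disables input, and IA_Interact calls ToggleSwitch, which sends Activate to ActorToActivate through BPI_Activable and stores IsDoorOpen.
; The interact event also swaps the keylock material and DoorON/DoorOFF visibility.
; Helper functions for camera switching and movement locking exist but are not called here.
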(event OnComponentBeginOverlap(Box)
  (params (OverlappedComponent :type Primitive%20Component%20Object%20Reference) (OtherActor :type Actor%20Object%20Reference) (OtherComp :type Primitive%20Component%20Object%20Reference) (OtherBodyIndex :type Integer) (bFromSweep :type Boolean) (SweepResult :type Hit%20Result%20Structure%20%28by%20ref%29))
  (Input|EnableInput (Game|GetPlayerController 0)))

(event OnComponentEndOverlap(Box)
  (params (OverlappedComponent :type Primitive%20Component%20Object%20Reference) (OtherActor :type Actor%20Object%20Reference) (OtherComp :type Primitive%20Component%20Object%20Reference) (OtherBodyIndex :type Integer))
  (Input|DisableInput (Game|GetPlayerController 0)))

(event Input|EnhancedActionEvents|EnhancedInputActionIA_Interact
  (params (ActionValue :type Boolean) (ElapsedSeconds :type Float%20%28double-precision%29) (TriggeredSeconds :type Float%20%28double-precision%29) (InputAction :type Input%20Action%20Object%20Reference :default "/Game/PlayerFolder/Input/Actions/IA_Interact.IA_Interact"))
  (:Started
    (if (Variables|Default|GetbIsDoorOpen)
      ;[1 1 1] IF door is open Close it
      (Utilities|ToggleSwitch false)
      (Rendering|Material|SetMaterial (Variables|Default|GetCube) 0 "/Engine/BasicShapes/MI_KeylockClosed.MI_KeylockClosed")
      (else
        ;[1 1 1] IF door is not open Open it
        (Utilities|ToggleSwitch true)
        (Rendering|Material|SetMaterial (Variables|Default|GetCube) 0 "/Engine/BasicShapes/MI_KeylockOpen.MI_KeylockOpen")))
    (if (Variables|Default|GetbIsDoorOpen)
      (Rendering|SetVisibility (Variables|Default|GetDoorOFF) false false)
      (Rendering|SetVisibility (Variables|Default|GetDoorON) true false)
      (else
        (Rendering|SetVisibility (Variables|Default|GetDoorON) false false)
        (Rendering|SetVisibility (Variables|Default|GetDoorOFF) true false)))))

(event EventBeginPlay
  (Rendering|Material|SetMaterial (Variables|Default|GetCube) 0 "/Engine/BasicShapes/MI_KeylockClosed.MI_KeylockClosed")
  (Rendering|SetVisibility (Variables|Default|GetDoorOFF) true false))

(fn ConstructionScript)

(fn IsDoorOpen
  (params (isOn :type Boolean))
  (if isOn
    _))

(fn ResetSequence)