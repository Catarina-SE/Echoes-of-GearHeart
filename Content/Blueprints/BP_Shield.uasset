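; Energy shield actor that shotgun projectiles wear down and temporarily disable.
; AbsorbArea overlaps drain TotalHealth; at zero the shield toggles collision off and scales its mesh to zero, then reactivates after a delay without restoring health.
; Base projectile hits briefly blink the dynamic material's colors red.
; Damage interface calls forward TakeDamage to BPCDamageSystem, while the other interface functions are stubs.
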(event OnComponentBeginOverlap(AbsorbArea)
  (params (OverlappedComponent :type Primitive%20Component%20Object%20Reference) (OtherActor :type Actor%20Object%20Reference) (OtherComp :type Primitive%20Component%20Object%20Reference) (OtherBodyIndex :type Integer) (bFromSweep :type Boolean) (SweepResult :type Hit%20Result%20Structure%20%28by%20ref%29))
  (Utilities|Casting|CastToBP_Projectile_Shotgun OtherActor)
  (if (Variables|Default|GetCanPlayHitReaction)
    (Variables|Default|SetPlayHitReaction true))
  (Variables|Default|SetTotalHealth (- (Variables|Default|GetTotalHealth) (Variables|Default|GetDisablingShots)))
  (if (<= (Variables|Default|GetTotalHealth) 0)
    (CallFunction|ReactivateShield)))

(event OnComponentHit(AbsorbArea)
  (params (HitComponent :type Primitive%20Component%20Object%20Reference) (OtherActor :type Actor%20Object%20Reference) (OtherComp :type Primitive%20Component%20Object%20Reference) (NormalImpulse :type Vector :default "0, 0, 0") (Hit :type Hit%20Result%20Structure%20%28by%20ref%29))
  (Utilities|Casting|CastToBP_Projectile_Base OtherActor)
  (CallFunction|BlinkShield))

(event Custom|BlinkShield
  (bind _shielddynamicmaterialref (Variables|Default|GetShieldDynamicMaterialRef))
  (bind _shielddynamicmaterialref_2 (Variables|Default|GetShieldDynamicMaterialRef))
  (Rendering|Material|SetVectorParameterValue _shielddynamicmaterialref_2 "Color" "(R=1.000000,G=0.000000,B=0.101925,A=1.000000)" :!class /Script/Engine.MaterialInstanceDynamic)
  (Rendering|Material|SetVectorParameterValue _shielddynamicmaterialref_2 "Color_Hexagon" "(R=1.000000,G=0.000000,B=0.101925,A=1.000000)" :!class /Script/Engine.MaterialInstanceDynamic)
  (Utilities|FlowControl|Delay 1.0)
  (Rendering|Material|SetVectorParameterValue _shielddynamicmaterialref "Color" (Variables|Default|GetShieldColor) :!class /Script/Engine.MaterialInstanceDynamic)
  (Rendering|Material|SetVectorParameterValue _shielddynamicmaterialref "Color_Hexagon" (Variables|Default|GetShieldColor2) :!class /Script/Engine.MaterialInstanceDynamic))

(event Custom|Activate
  (Utilities|IsValid self
    (:Is%20Valid
      (Collision|SetCollisionEnabled (Variables|Default|GetAbsorbArea) "QueryOnly")
      (CallFunction|ExpandShield))
    (:Is%20Not%20Valid
      (Development|PrintString "Shield is not enabled"))))

(event Custom|Deactivate
  (Utilities|IsValid self
    (:Is%20Valid
      (Collision|SetCollisionEnabled (Variables|Default|GetAbsorbArea) "NoCollision")
      (CallFunction|ShrinkShield))
    (:Is%20Not%20Valid
      (Development|PrintString "Shield is not enabled"))))

(event Custom|ShrinkShield
  (Transformation|SetRelativeScale3D (Variables|Default|GetStaticMesh) "0, 0, 0"))

(event Custom|ExpandShield
  (Transformation|SetRelativeScale3D (Variables|Default|GetStaticMesh) "0.152500,1.000000,0.250000"))

(event Custom|ReactivateShield
  (CallFunction|Deactivate)
  (Utilities|FlowControl|Delay 0.1)
  (Variables|Default|SetPlayHitReaction false)
  (Utilities|FlowControl|Delay (Variables|Default|GetTimetoReactivateShield))
  (CallFunction|Activate)
  (Variables|Default|SetTotalHealth (Variables|Default|GetTotalHealth)))

(event EventBeginPlay)

(event Collision|EventActorBeginOverlap
  (params (OtherActor :type Actor%20Object%20Reference)))

(fn ConstructionScript
  (Variables|Default|SetShieldHealth (Variables|Default|GetShieldHealth))
  (bind _returnvalue (Rendering|Material|CreateDynamicMaterialInstance (Variables|Default|GetStaticMesh) 0 "/Game/Materials/MI_Shield_Front.MI_Shield_Front" "None" :!class /Script/Engine.PrimitiveComponent))
  (bind _output_get (Variables|Default|SetShieldDynamicMaterialRef _returnvalue))
  (Rendering|Material|SetVectorParameterValue _output_get "Color" (Variables|Default|GetShieldColor) :!class /Script/Engine.MaterialInstanceDynamic)
  (Rendering|Material|SetVectorParameterValue _output_get "Color_Hexagon" (Variables|Default|GetShieldColor2) :!class /Script/Engine.MaterialInstanceDynamic))

(fn GetCurrentHealth
  (return 0.0))

(fn GetIdealRange
  (return 0.0 0.0))

(fn GetMaxHealth
  (return 0.0))

(fn GetPatrolRoute
  (return 0))

(fn Heal
  (params (Amount :type Float%20%28double-precision%29))
  (return 0.0))

(fn IsDead
  (return false))

(fn SetMovementSpeed
  (params (Speed :type E_MovementSpeed%20Enum :default "NewEnumerator0"))
  (return 0.0))

(fn TakeDamage
  (params (DamageInfo :type S%20Damage%20Info%20Structure))
  (bind _wasdamaged (Default|TakeDamage (Variables|Default|GetBPC_DamageSystem) DamageInfo))
  (return _wasdamaged))